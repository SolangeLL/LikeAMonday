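; BP_Zombie is a zombie enemy character that chases and attacks the player, takes damage and dies.
; PawnSensing triggers an AI move to the player, and arrival starts an attack montage guarded against re-entry.
; A montage notify damages whichever player the detection overlap has stored.
; Damage goes through a health component, playing a hit reaction or a death animation with timed destruction, and a health bar widget references the zombie.
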(event OnSeePawn(PawnSensing)
  (params (Pawn :type Pawn%20Object%20Reference))
  ;[1 0.6353 0.4745] Player to chase detection
  (Utilities|Casting|CastToBP_Player Pawn)
  (CallFunction|ChasePlayer)
  (Utilities|FlowControl|Delay 5.0)
  (if (Variables|/Script/AIModule.PawnSensingComponent|GetbSeePawns (Variables|Default|GetPawnSensing))
    (Components|Movement|StopMovementImmediately (Variables|Character|GetCharacterMovement))))

(event OnComponentBeginOverlap(PlayerDetection)
  (params (OverlappedComponent :type Primitive%20Component%20Object%20Reference) (OtherActor :type Actor%20Object%20Reference) (OtherComp :type Primitive%20Component%20Object%20Reference) (OtherBodyIndex :type Integer) (bFromSweep :type Boolean) (SweepResult :type Hit%20Result%20Structure%20%28by%20ref%29))
  ;[1 0.6353 0.4745] Player in attack zone detection
  (bind _asbp_player (Utilities|Casting|CastToBP_Player OtherActor))
  (Variables|Default|SetPlayer%20In%20Zone _asbp_player))

(event OnComponentEndOverlap(PlayerDetection)
  (params (OverlappedComponent :type Primitive%20Component%20Object%20Reference) (OtherActor :type Actor%20Object%20Reference) (OtherComp :type Primitive%20Component%20Object%20Reference) (OtherBodyIndex :type Integer))
  ;[1 0.6353 0.4745] Player in attack zone detection
  (Utilities|Casting|CastToBP_Player OtherActor)
  (Variables|Default|SetPlayer%20In%20Zone 0))

(event Custom|Chase%20Player
  ;[0.03922 0.1255 0.149] Chase player event
  (if (not (Variables|Default|GetIsDead))
    (bind _asbp_player (Utilities|Casting|CastToBP_Player (Game|GetPlayerCharacter 0)))
    (AI|AIMoveTo self "0, 0, 0" _asbp_player 7e+01 false
      (:OnSuccess
        (CallFunction|AttackPlayer)))))

(event Custom|Attack%20Player
  (bind _player_in_zone (Variables|Default|GetPlayer%20In%20Zone))
  ;[0.03922 0.1255 0.149] Attack player event
  (if (not (Variables|Default|GetIs%20Attacking))
    (Utilities|FlowControl|Sequence
      (:then_0
        ;;[0.149 0.149 0.149 0.8471] Stop moving
        (Variables|Default|SetIs%20Attacking true)
        (bind _asaicontroller (Utilities|Casting|CastToAIController (Pawn|GetController)))
        (AI|ClearFocus _asaicontroller)
        (Components|Movement|StopMovementImmediately (Variables|Character|GetCharacterMovement)))
      (:then_1
        ;;[0.149 0.149 0.149 0.8471] Play attack animation
        (Animation|Montage|PlayMontage (Variables|Character|GetMesh) "/Game/Zombies/Animations/Montages/ZombieAttack_Montage.ZombieAttack_Montage"
          (:then
            (Utilities|FlowControl|Delay 2.63))
          (:OnCompleted
            (Variables|Default|SetIs%20Attacking false :!label _label))
          (:OnBlendOut
            (goto _label))
          (:OnInterrupted
            (goto _label))
          (:OnNotifyBegin
            (if (not (== _player_in_zone 0))
              (Default|TakeDamage _player_in_zone (Variables|Default|GetDamage)))))))))

(event EventTick
  (params (DeltaSeconds :type Float%20%28single-precision%29))
  (if (Variables|Default|GetIsDead)
    (Utilities|Time|SetTimerbyEvent 0 0.0)))

(event EventBeginPlay
  (bind _aszombie_health (Utilities|Casting|CastToZombie_Health (UserInterface|GetUserWidgetObject (Variables|Default|GetHealthbar))))
  (Variables|/Game/Zombies/Zombie_Health.Zombie_Health_C|SetZombieRef _aszombie_health self))

(fn ConstructionScript)

(fn TakeDamage
  (params (Damage :type Float%20%28double-precision%29))
  (bind _mesh (Variables|Character|GetMesh))
  (bind _bisdead (Class|AAAHealthSystemComponent|ReduceHealth (Variables|Default|GetAAA_HealthSystem) Damage))
  (if _bisdead
    (Variables|Default|SetIsDead true)
    (Components|Animation|SetAnimation _mesh 0)
    (Components|Animation|PlayAnimation _mesh "/Game/Zombies/Animations/ZombieDie.ZombieDie" false)
    (Components|Activation|SetActive (Variables|Character|GetCharacterMovement) false false)
    (Utilities|Time|SetTimerbyFunctionName 0 "Die" 3.0)
    (else
      (Animation|PlayAnimMontage "/Game/Zombies/Animations/Montages/ZombieHit_Montage.ZombieHit_Montage" 1.0 "None"))))

(fn Die
  (Actor|DestroyActor))