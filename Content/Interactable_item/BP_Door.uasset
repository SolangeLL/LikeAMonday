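; BP_Door is an interactable hinged door that toggles open and closed when its Interact event fires.
; BeginPlay caches the Door component's starting rotation as closed and adds 90 degrees of yaw for the open target.
; Tick eases the door's relative rotation toward the active target with RInterpTo at RotationSpeed, interpolating every frame rather than using a timeline.
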(event EventBeginPlay
  (bind _output_get (Variables|Default|SetClosedRotation (Variables|/Script/Engine.SceneComponent|GetRelativeRotation (Variables|Default|Getdoor))))
  (Variables|Default|SetOpenRotation (Math|Rotator|MakeRotator (.roll _output_get) (.pitch _output_get) (+ (.yaw _output_get) 9e+01))))

(event Collision|EventActorBeginOverlap
  (params (OtherActor :type Actor%20Object%20Reference)))

(event EventTick
  (params (DeltaSeconds :type Float%20%28single-precision%29))
  (bind _rotationspeed (Variables|Default|GetRotationSpeed))
  (bind _door (Variables|Default|Getdoor))
  (bind _relativerotation (Variables|/Script/Engine.SceneComponent|GetRelativeRotation _door))
  (if (Variables|Default|GetIsOpen)
    (Transformation|SetRelativeRotation (Variables|Default|Getdoor) (Math|Interpolation|RInterpTo _relativerotation (Variables|Default|GetOpenRotation) DeltaSeconds _rotationspeed) false false)
    (else
      (Transformation|SetRelativeRotation (Variables|Default|Getdoor) (Math|Interpolation|RInterpTo _relativerotation (Variables|Default|GetClosedRotation) DeltaSeconds _rotationspeed) false false))))

(event EventInteract
  (Variables|Default|SetIsOpen (not (Variables|Default|GetIsOpen))))

(fn ConstructionScript)