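; Inventory component that stores weapons in a map of slots keyed by weapon type.
; SetWeaponInSlot writes a weapon into its slot and passes it to EquipNewWeapon on player 0's BP_Player pawn.
; GetWeaponByType looks up a slot, while EquipWeapon rebuilds the stored struct with its IsEquipped flag inverted, so it acts as a toggle.
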(event EventBeginPlay)

(event EventTick
  (params (DeltaSeconds :type Float%20%28single-precision%29)))

(fn SetWeaponinSlot
  (params (Weapon :type Weapon%20Data%20Structure) (WeaponType :type E_WeaponType%20Enum :default "NewEnumerator0"))
  (Utilities|Map|Add (Variables|Default|GetWeaponSlots) WeaponType Weapon)
  (bind _asbp_player (Utilities|Casting|CastToBP_Player (Game|Player|GetPlayerPawn 0)))
  (Default|EquipNewWeapon _asbp_player Weapon))

(fn GetWeaponbyType
  (params (Type :type E_WeaponType%20Enum :default "NewEnumerator0"))
  (return (.Value (Utilities|Map|Find (Variables|Default|GetWeaponSlots) Type))))

(fn EquipWeapon
  (params (Type :type E_WeaponType%20Enum :default "NewEnumerator0"))
  (bind _weaponslots (Variables|Default|GetWeaponSlots))
  (bind _value (Utilities|Map|Find _weaponslots Type))
  (bind (_type _name _attackmontage _damage _speed _mesh _drawmontage _sheathemontage _equippedsocket _unequippedsocket _isequipped _uimat _maxammo _blueprint) (Utilities|Struct|BreakWeaponData _value))
  (Utilities|Map|Add (Variables|Default|GetWeaponSlots) Type (Utilities|Struct|MakeWeaponData _type _name _attackmontage _damage _speed _mesh _drawmontage _sheathemontage _equippedsocket _unequippedsocket (not _isequipped) _uimat _maxammo _blueprint "(ProjectileMesh_2_4F6B16D64AFBA38E8B57D0A628AA64AA=None,Speed_13_2FCEDEFA4610E07B9F9A0EAB534E2282=0.000000,GravityScale_14_8402D76446F8F19BF6A8C7B98B8876F1=0.000000,Damage_16_A603EB1343D5D7B00838108AFD95D2FA=0.000000,Lifetime_17_1A7E20924BCD871661CD2C83A692E721=0.000000,ShootSound_19_9A78B3A94FBC1C94AA3F78B835E60F63=None,HitSound_22_625563AE4FA550CA32FE8785FD7FC77F=None)")))