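; BP_Projectile is a data-driven projectile actor that plays a sound on impact and destroys itself shortly afterwards.
; Init stores the passed projectile data, then uses it to set the static mesh, max speed and gravity scale, and makes the mesh the movement component's updated component.
; A mesh hit plays the data's hit sound in 2D and applies no damage.
; The construction script only prints a debug string.
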(event OnComponentHit(ProjectileMesh)
  (params (HitComponent :type Primitive%20Component%20Object%20Reference) (OtherActor :type Actor%20Object%20Reference) (OtherComp :type Primitive%20Component%20Object%20Reference) (NormalImpulse :type Vector :default "0, 0, 0") (Hit :type Hit%20Result%20Structure%20%28by%20ref%29))
  (Audio|PlaySound2D (.HitSound (Utilities|Struct|BreakFProjectileData (Variables|Default|GetProjectileData))) 1.0 1.0 0.0 0 0)
  (Utilities|FlowControl|Delay 0.2)
  (Actor|DestroyActor))

(event EventBeginPlay)

(event Collision|EventActorBeginOverlap
  (params (OtherActor :type Actor%20Object%20Reference)))

(event EventTick
  (params (DeltaSeconds :type Float%20%28single-precision%29)))

(fn ConstructionScript
  (Development|PrintString "Construct bullet"))

(fn Init
  (params (Projectile :type F%20Projectile%20Data%20Structure))
  (bind _projectilemovement (Variables|Default|GetProjectileMovement))
  (bind _output_get (Variables|Default|SetProjectileData Projectile))
  (Components|StaticMesh|SetStaticMesh (Variables|Default|GetProjectile%20Mesh) (.ProjectileMesh (Utilities|Struct|BreakFProjectileData _output_get)))
  (Variables|/Script/Engine.ProjectileMovementComponent|SetMaxSpeed _projectilemovement (.Speed (Utilities|Struct|BreakFProjectileData _output_get)))
  (Variables|/Script/Engine.ProjectileMovementComponent|SetProjectileGravityScale _projectilemovement (.GravityScale (Utilities|Struct|BreakFProjectileData _output_get)))
  (Components|Movement|SetUpdatedComponent _projectilemovement (Variables|Default|GetProjectile%20Mesh)))