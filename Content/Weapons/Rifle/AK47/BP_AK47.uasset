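; BP_AK47 is the AK47 rifle weapon Blueprint, a child class that supplies the rifle's firing behavior.
; Its Attack override calls Shoot on FireWeapon, passing the projectile from its Weapon data and the world transform of BulletSpawn, then runs the parent Attack.
; The event graph holds only disabled default events, and the construction script just calls the parent.
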(event EventBeginPlay
  (|CallParentFunction) ; This node is disabled and will not be called.\nDrag off pins to build functionality.
)

(event Collision|EventActorBeginOverlap
  (params (OtherActor :type Actor%20Object%20Reference))
  (|CallParentFunction OtherActor) ; This node is disabled and will not be called.\nDrag off pins to build functionality.
)

(event EventTick
  (params (DeltaSeconds :type Float%20%28single-precision%29))
  (|CallParentFunction DeltaSeconds) ; This node is disabled and will not be called.\nDrag off pins to build functionality.
)

(fn ConstructionScript
  (|CallParentFunction))

(fn Attack
  (Default|Shoot (Variables|Default|GetFireWeapon) (.Projectile (Utilities|Struct|BreakWeaponData (Variables|Default|GetWeapon))) (Transformation|GetWorldTransform (Variables|Default|GetBullet%20Spawn)))
  (|CallParentFunction))