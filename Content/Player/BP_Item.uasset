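; BP_Item is a weapon item that mounts itself on the player's body when picked up.
; The construction script applies WeaponModel to the Item static mesh.
; PickingUp casts player 0's character to BP_PlayerTest and, after a tiny delay, calls WeaponSlot.
; WeaponSlot snaps the Item component, not the actor, to a melee, gun or rifle socket by Slot and stores it in the matching player variable.
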(event EventPickingUp
  (bind _asbp_player_test (Utilities|Casting|CastToBP_PlayerTest (Game|GetPlayerCharacter 0)))
  (Variables|Default|SetPlayer _asbp_player_test)
  (Utilities|FlowControl|Delay 0.001)
  (Utilities|WeaponSlot))

(fn ConstructionScript
  (Components|StaticMesh|SetStaticMesh (Variables|Default|GetItem) (Variables|Default|GetWeaponModel)))