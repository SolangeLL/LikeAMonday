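; Test player character for mouse-aimed play: Enhanced Input movement relative to control yaw, smooth turning toward the cursor hit point, and X-key speed toggle.
; Draw inputs play montages whose notifies move melee, gun or rifle between holster and hand sockets, setting a shared equipped flag and slot.
; Attack picks a montage by slot, but the rifle branch repeats the gun's check, so never fires.
; Pickup checks overlapping actors' interface but does nothing further.
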(event Input|EnhancedActionEvents|EnhancedInputActionIA_PickUp
  (params (ActionValue :type Boolean) (ElapsedSeconds :type Float%20%28double-precision%29) (TriggeredSeconds :type Float%20%28double-precision%29) (InputAction :type Input%20Action%20Object%20Reference :default "/Game/Player/Inputs/Actions/IA_PickUp.IA_PickUp"))
  ;[0.15 0.15 0.15 0.5] Pick Up System
  (:Started
    (CallFunction|PickingUp)))

(event Input|EnhancedActionEvents|EnhancedInputActionIA_Draw3
  (params (ActionValue :type Boolean) (ElapsedSeconds :type Float%20%28double-precision%29) (TriggeredSeconds :type Float%20%28double-precision%29) (InputAction :type Input%20Action%20Object%20Reference :default "/Game/Player/Inputs/Actions/IA_Draw3.IA_Draw3"))
  ;[1 1 1 0.5] Draw Rifle
  (if (Variables|Default|GetIsEquipped)
    (Animation|Montage|PlayMontage (Variables|Character|GetMesh) "/Game/Player/Animations/Rifle/SheatheRifle_Montage.SheatheRifle_Montage"
      (:OnNotifyBegin
        (Transformation|AttachComponentToComponent (Variables|Default|GetRifle) (Variables|Character|GetMesh) "back_rifle" "SnapToTarget" "SnapToTarget" "SnapToTarget" true)
        (Variables|Default|SetIsEquipped false)
        (Variables|Default|SetWeaponSlot 0)))
    (else
      (Animation|Montage|PlayMontage (Variables|Character|GetMesh) "/Game/Player/Animations/Rifle/DrawRifle_Montage.DrawRifle_Montage"
        (:OnNotifyBegin
          (Transformation|AttachComponentToComponent (Variables|Default|GetRifle) (Variables|Character|GetMesh) "rifle" "SnapToTarget" "SnapToTarget" "SnapToTarget" true)
          (Variables|Default|SetIsEquipped true)
          (Variables|Default|SetWeaponSlot 3))))))

(event Input|EnhancedActionEvents|EnhancedInputActionIA_Attack
  (params (ActionValue :type Boolean) (ElapsedSeconds :type Float%20%28double-precision%29) (TriggeredSeconds :type Float%20%28double-precision%29) (InputAction :type Input%20Action%20Object%20Reference :default "/Game/Player/Inputs/Actions/IA_Attack.IA_Attack"))
  (:Started
    (if (== (Variables|Default|GetWeaponSlot) 1)
      (Animation|Montage|PlayMontage (Variables|Character|GetMesh) "/Game/Player/Animations/Melee/AttackHammer_Montage.AttackHammer_Montage")
      (elif (== (Variables|Default|GetWeaponSlot) 2)
        (Animation|Montage|PlayMontage (Variables|Character|GetMesh) "/Game/Player/Animations/Gun/GunShoot_Montage.GunShoot_Montage")
        (elif (== (Variables|Default|GetWeaponSlot) 2)
          (Animation|Montage|PlayMontage (Variables|Character|GetMesh) "/Game/Player/Animations/Rifle/RifleShoot_Montage.RifleShoot_Montage"))))))

(event Input|EnhancedActionEvents|EnhancedInputActionIA_Move1
  (params (ActionValue :type Vector%202D%20Structure) (ElapsedSeconds :type Float%20%28double-precision%29) (TriggeredSeconds :type Float%20%28double-precision%29) (InputAction :type Input%20Action%20Object%20Reference :default "/Game/Player/Inputs/Actions/IA_Move1.IA_Move1"))
  (bind _returnvalue (Pawn|GetControlRotation :!class /Script/Engine.Pawn))
  ;[0 0 0 0.5] Move Right / Left
  (Pawn|Input|AddMovementInput (Math|Vector|GetRightVector (Math|Rotator|MakeRotator (.roll _returnvalue) 0.0 (.yaw _returnvalue))) (.x ActionValue) false)
  ;[0 0 0 0.5] Move Forward / Backwards
  (Pawn|Input|AddMovementInput (Math|Vector|GetForwardVector (Math|Rotator|MakeRotator 0.0 0.0 (.yaw (Pawn|GetControlRotation :!class /Script/Engine.Pawn)))) (.y ActionValue) false))

(event Input|EnhancedActionEvents|EnhancedInputActionIA_Draw1
  (params (ActionValue :type Boolean) (ElapsedSeconds :type Float%20%28double-precision%29) (TriggeredSeconds :type Float%20%28double-precision%29) (InputAction :type Input%20Action%20Object%20Reference :default "/Game/Player/Inputs/Actions/IA_Draw1.IA_Draw1"))
  ;[1 1 1 0.5] Draw Melee Weapon
  (:Started
    (if (Variables|Default|GetIsEquipped)
      (Animation|Montage|PlayMontage (Variables|Character|GetMesh) "/Game/Player/Animations/Melee/SheatheMeleeWeapon_Montage.SheatheMeleeWeapon_Montage"
        (:OnNotifyBegin
          (Transformation|AttachComponentToComponent (Variables|Default|GetMeleeWeapon) (Variables|Character|GetMesh) "holster_melee" "SnapToTarget" "SnapToTarget" "SnapToTarget" true)
          (Variables|Default|SetIsEquipped false)
          (Variables|Default|SetWeaponSlot 0)))
      (else
        (Animation|Montage|PlayMontage (Variables|Character|GetMesh) "/Game/Player/Animations/Melee/DrawMeleeWeapon_Montage.DrawMeleeWeapon_Montage"
          (:OnNotifyBegin
            (Transformation|AttachComponentToComponent (Variables|Default|GetMeleeWeapon) (Variables|Character|GetMesh) "melee" "SnapToTarget" "SnapToTarget" "SnapToTarget" true)
            (Variables|Default|SetIsEquipped true)
            (Variables|Default|SetWeaponSlot 1)))))))

(event Input|EnhancedActionEvents|EnhancedInputActionIA_Draw2
  (params (ActionValue :type Boolean) (ElapsedSeconds :type Float%20%28double-precision%29) (TriggeredSeconds :type Float%20%28double-precision%29) (InputAction :type Input%20Action%20Object%20Reference :default "/Game/Player/Inputs/Actions/IA_Draw2.IA_Draw2"))
  ;[1 1 1 0.5] Draw Gun
  (:Started
    (if (Variables|Default|GetIsEquipped)
      (Animation|Montage|PlayMontage (Variables|Character|GetMesh) "/Game/Player/Animations/Gun/SheatheGun_Montage.SheatheGun_Montage"
        (:OnNotifyBegin
          (Transformation|AttachComponentToComponent (Variables|Default|GetGun) (Variables|Character|GetMesh) "holster_gun" "SnapToTarget" "SnapToTarget" "SnapToTarget" true)
          (Variables|Default|SetIsEquipped false)
          (Variables|Default|SetWeaponSlot 0)))
      (else
        (Animation|Montage|PlayMontage (Variables|Character|GetMesh) "/Game/Player/Animations/Gun/DrawGun_Montage.DrawGun_Montage"
          (:OnNotifyBegin
            (Transformation|AttachComponentToComponent (Variables|Default|GetGun) (Variables|Character|GetMesh) "gun" "SnapToTarget" "SnapToTarget" "SnapToTarget" true)
            (Variables|Default|SetIsEquipped true)
            (Variables|Default|SetWeaponSlot 2)))))))

(event EventTick
  (params (DeltaSeconds :type Float%20%28single-precision%29))
  (bind _returnvalue (Transformation|GetActorRotation))
  ;[0.15 0.15 0.15 0.5] Set Player face cursor
  (Transformation|SetActorRotation (Math|Rotator|MakeRotator (.roll _returnvalue) (.pitch _returnvalue) (.yaw (Class|KismetMathLibrary|RInterptoConstant (Transformation|GetActorRotation) (Math|Rotator|FindLookatRotation (+ "" "") (- (.ImpactPoint (Collision|BreakHitResult (.HitResult (Game|Player|GetHitResultUnderCursorbyChannel (Game|GetPlayerController 0) "TraceTypeQuery1" true)))) (Transformation|GetActorLocation))) (Utilities|Time|GetWorldDeltaSeconds) (Variables|Default|GetInterp%20Speed))))))

(event EventBeginPlay
  ;[0.05098 0.05098 0.05098] Add Mapping Context
  (bind _asbp_player_controller (Utilities|Casting|CastToBP_PlayerController (Pawn|GetController)))
  (Utilities|IsValid (PlayerController|LocalPlayerSubsystems|GetEnhancedInputLocalPlayerSubsystem _asbp_player_controller)
    (:Is%20Valid
      (Input|AddMappingContext (PlayerController|LocalPlayerSubsystems|GetEnhancedInputLocalPlayerSubsystem _asbp_player_controller) "/Game/Player/Inputs/IMC_PlayerTest.IMC_PlayerTest" 0 "(bIgnoreAllPressedKeysUntilRelease=True,bForceImmediately=False,bNotifyUserSettings=False)")
      (Variables|/Script/Engine.PlayerController|SetbShowMouseCursor (Game|GetPlayerController 0) true))))

(event EventPickingUp
  ;[0.15 0.15 0.15 0.5] Pick Up System
  (bind _array_element (Utilities|Array|ForEachLoopwithBreak (Collision|GetOverlappingActors "/Script/Engine.Actor" :!class /Script/Engine.Actor))
    (:LoopBody
      (if (Utilities|DoesObjectImplementInterface _array_element "/Game/Player/BPI_PickUp.BPI_PickUp_C")
        _))))

(event Input|KeyboardEvents|X
  (params (Key :type Key%20Structure :default "None"))
  (bind _charactermovement (Variables|Character|GetCharacterMovement))
  (:Released
    (if (== (Variables|/Script/Engine.CharacterMovementComponent|GetMaxWalkSpeed (Variables|Character|GetCharacterMovement)) 2e+02)
      (Variables|/Script/Engine.CharacterMovementComponent|SetMaxWalkSpeed _charactermovement 6e+02)
      (else
        (Variables|/Script/Engine.CharacterMovementComponent|SetMaxWalkSpeed _charactermovement 2e+02)))))

(fn ConstructionScript)