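; Player character that turns toward the mouse cursor, moves via Enhanced Input, and fights unarmed or with melee, gun and rifle weapons.
; Slot inputs fetch Inventory weapons, then draw or sheathe them, swapping mesh sockets on montage notifies.
; Attacks play random unarmed or weapon montages behind a timed lock; damage feeds the health component.
; Possession creates the HUD; temporary keys fill inventory slots, and pickup's interface message is unwired.
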(event Custom|Sheathe%20Weapon
  ;[1 1 1 0.5] Weapon Inventory System
  ;;[0.01961 0.05882 0 0.502] Sheath Weapon
  (Animation|Montage|PlayMontage (Variables|Character|GetMesh) (.SheatheMontage (Utilities|Struct|BreakWeaponData (Variables|Combat|GetCurrentWeapon)))
    (:OnNotifyBegin
      (bind _weapon_mesh (CallFunction|GetWeaponMeshbyType (.Type (Utilities|Struct|BreakWeaponData (Variables|Combat|GetCurrentWeapon)))))
      (Transformation|AttachComponentToComponent _weapon_mesh (Variables|Character|GetMesh) (.UnequippedSocket (Utilities|Struct|BreakWeaponData (Variables|Combat|GetCurrentWeapon))) "SnapToTarget" "SnapToTarget" "SnapToTarget" true)
      (Variables|Combat|SetIsEquipped false)
      (Default|EquipWeapon (Variables|Default|GetInventory) (.Type (Utilities|Struct|BreakWeaponData (Variables|Combat|GetCurrentWeapon))))
      (Variables|Combat|SetCurrentWeapon "(Type_2_DC035945415C65414341A89D8695E827=NewEnumerator0,Name_23_9F774E36402659E0E33F4CAEF4BF0E04=\"\",AttackMontage_24_F0C4FB1A45586646FF47E1AB01CAD0C7=None,Damage_25_67E234574A0C52D3B3C5A7890181090E=0.000000,Speed_22_1B28431A4BA63B29E6F20A93148BC307=0.000000,Mesh_28_DF7426E04EA62200147BEDB71847F082=None,DrawMontage_33_1368AC4E4FD6F8595F54EB820216956C=None,SheatheMontage_34_0CA10AE448688B085CA42D82C1E35E18=None,EquippedSocket_41_68CAC5334B8DE160778E1483B751AFBC=\"\",UnequippedSocket_42_C0DD2404464AB146AEC5AFA54DB6FEEB=\"\",IsEquipped_44_ED4119404BE92BA34C6172AE93BB77EC=False)"))))

(event Custom|Draw%20Weapon
  ;[1 1 1 0.5] Weapon Inventory System
  ;;[0.01961 0.05882 0 0.502] Draw Weapon
  (Animation|Montage|PlayMontage (Variables|Character|GetMesh) (.DrawMontage (Utilities|Struct|BreakWeaponData (Variables|Combat|GetPendingWeapon)))
    (:OnNotifyBegin
      (bind _weapon_mesh (CallFunction|GetWeaponMeshbyType (.Type (Utilities|Struct|BreakWeaponData (Variables|Combat|GetPendingWeapon)))))
      (Transformation|AttachComponentToComponent _weapon_mesh (Variables|Character|GetMesh) (.EquippedSocket (Utilities|Struct|BreakWeaponData (Variables|Combat|GetPendingWeapon))) "SnapToTarget" "SnapToTarget" "SnapToTarget" true)
      (Variables|Combat|SetIsEquipped true)
      (bind _output_get (Variables|Combat|SetCurrentWeapon (Variables|Combat|GetPendingWeapon)))
      (Default|EquipWeapon (Variables|Default|GetInventory) (.Type (Utilities|Struct|BreakWeaponData _output_get)))
      (Variables|Combat|SetPendingWeapon ""))))

(event Custom|Update%20Weapon%20State
  ;[1 1 1 0.5] Weapon Inventory System
  ;;[0.15 0.15 0.15 0.5] Update weapon state to see if we have to draw, sheathe or do nothing
  (if (not (== (.Mesh (Utilities|Struct|BreakWeaponData (Variables|Combat|GetPendingWeapon))) 0))
    (if (Variables|Combat|GetIsEquipped)
      (CallFunction|SheatheWeapon)
      (else
        (CallFunction|DrawWeapon)))))

(event Custom|Client%20Create%20HUD
  (params (Object :type Controller%20Object%20Reference))
  (bind _asbp_player_controller (Utilities|Casting|CastToBP_PlayerController Object))
  (bind _output_get (Variables|Default|SetAs%20BP%20controller _asbp_player_controller))
  (Default|CreateHUD _output_get))

(event Input|EnhancedActionEvents|EnhancedInputActionIA_PickUp
  (params (ActionValue :type Boolean) (ElapsedSeconds :type Float%20%28double-precision%29) (TriggeredSeconds :type Float%20%28double-precision%29) (InputAction :type Input%20Action%20Object%20Reference :default "/Game/Player/Inputs/Actions/IA_PickUp.IA_PickUp"))
  ;[0.15 0.15 0.15 0.5] Pick Up System
  (:Started
    (CallFunction|PickingUp)))

(event Input|EnhancedActionEvents|EnhancedInputActionIA_Draw3
  (params (ActionValue :type Boolean) (ElapsedSeconds :type Float%20%28double-precision%29) (TriggeredSeconds :type Float%20%28double-precision%29) (InputAction :type Input%20Action%20Object%20Reference :default "/Game/Player/Inputs/Actions/IA_Draw3.IA_Draw3"))
  ;[0.15 0.15 0.15 0.5] Weapon Selection
  (CallFunction|EquipWeaponbyType "NewEnumerator2")
  (CallFunction|UpdateWeaponState))

(event Input|EnhancedActionEvents|EnhancedInputActionIA_Attack
  (params (ActionValue :type Boolean) (ElapsedSeconds :type Float%20%28double-precision%29) (TriggeredSeconds :type Float%20%28double-precision%29) (InputAction :type Input%20Action%20Object%20Reference :default "/Game/Player/Inputs/Actions/IA_Attack.IA_Attack"))
  ;[1 0.375 0.375 0.5] Attack System
  (if (Variables|Combat|GetIsEquipped)
    (Utilities|AttackwithWeapon)
    (else
      (Utilities|AttackwithNoWeapon))))

(event Input|EnhancedActionEvents|EnhancedInputActionIA_Move1
  (params (ActionValue :type Vector%202D%20Structure) (ElapsedSeconds :type Float%20%28double-precision%29) (TriggeredSeconds :type Float%20%28double-precision%29) (InputAction :type Input%20Action%20Object%20Reference :default "/Game/Player/Inputs/Actions/IA_Move1.IA_Move1"))
  (bind _returnvalue (Pawn|GetControlRotation :!class /Script/Engine.Pawn))
  ;[0 0 0 0.5] Move Right / Left
  (Pawn|Input|AddMovementInput (Math|Vector|GetRightVector (Math|Rotator|MakeRotator (.roll _returnvalue) 0.0 (.yaw _returnvalue))) (.x ActionValue) false)
  ;[0 0 0 0.5] Move Forward / Backwards
  (Pawn|Input|AddMovementInput (Math|Vector|GetForwardVector (Math|Rotator|MakeRotator 0.0 0.0 (.yaw (Pawn|GetControlRotation :!class /Script/Engine.Pawn)))) (.y ActionValue) false))

(event Input|EnhancedActionEvents|EnhancedInputActionIA_Draw1
  (params (ActionValue :type Boolean) (ElapsedSeconds :type Float%20%28double-precision%29) (TriggeredSeconds :type Float%20%28double-precision%29) (InputAction :type Input%20Action%20Object%20Reference :default "/Game/Player/Inputs/Actions/IA_Draw1.IA_Draw1"))
  ;[0.15 0.15 0.15 0.5] Weapon Selection
  (:Started
    (CallFunction|EquipWeaponbyType "NewEnumerator3")
    (CallFunction|UpdateWeaponState)))

(event Input|EnhancedActionEvents|EnhancedInputActionIA_Draw2
  (params (ActionValue :type Boolean) (ElapsedSeconds :type Float%20%28double-precision%29) (TriggeredSeconds :type Float%20%28double-precision%29) (InputAction :type Input%20Action%20Object%20Reference :default "/Game/Player/Inputs/Actions/IA_Draw2.IA_Draw2"))
  ;[0.15 0.15 0.15 0.5] Weapon Selection
  (CallFunction|EquipWeaponbyType "NewEnumerator1")
  (CallFunction|UpdateWeaponState))

(event EventTick
  (params (DeltaSeconds :type Float%20%28single-precision%29))
  (bind _returnvalue (Transformation|GetActorRotation))
  ;[0.15 0.15 0.15 0.5] Set Player face cursor
  (Transformation|SetActorRotation (Math|Rotator|MakeRotator (.roll _returnvalue) (.pitch _returnvalue) (.yaw (Class|KismetMathLibrary|RInterptoConstant (Transformation|GetActorRotation) (Math|Rotator|FindLookatRotation (+ "" "") (- (.ImpactPoint (Collision|BreakHitResult (.HitResult (Game|Player|GetHitResultUnderCursorbyChannel (Game|GetPlayerController 0) "TraceTypeQuery1" true)))) (Transformation|GetActorLocation))) (Utilities|Time|GetWorldDeltaSeconds) (Variables|Default|GetInterp%20Speed))))))

(event EventBeginPlay
  ;[0.05098 0.05098 0.05098] Add Mapping Context
  (bind _asbp_player_controller (Utilities|Casting|CastToBP_PlayerController (Pawn|GetController)))
  (Utilities|IsValid (PlayerController|LocalPlayerSubsystems|GetEnhancedInputLocalPlayerSubsystem _asbp_player_controller)
    (:Is%20Valid
      (Input|AddMappingContext (PlayerController|LocalPlayerSubsystems|GetEnhancedInputLocalPlayerSubsystem _asbp_player_controller) "/Game/Player/Inputs/IMC_PlayerTest.IMC_PlayerTest" 0 "(bIgnoreAllPressedKeysUntilRelease=True,bForceImmediately=False,bNotifyUserSettings=False)")
      (Variables|/Script/Engine.PlayerController|SetbShowMouseCursor (Game|GetPlayerController 0) true))))

(event EventPickingUp
  ;[0.15 0.15 0.15 0.5] Pick Up System
  (bind _array_element (Utilities|Array|ForEachLoopwithBreak (Collision|GetOverlappingActors "/Script/Engine.Actor" :!class /Script/Engine.Actor))
    (:LoopBody
      (if (Utilities|DoesObjectImplementInterface _array_element "/Game/Player/BPI_PickUp.BPI_PickUp_C")
        _))))

(event EventPossessed
  (params (NewController :type Controller%20Object%20Reference))
  (CallFunction|ClientCreateHUD NewController))

(event Input|KeyboardEvents|N
  (params (Key :type Key%20Structure :default "None"))
  ;[0.01932 0 0.15 0.5] TEMPORARY Assign weapons in inventory
  (:Released
    (bind _returnvalue (Utilities|GetDataTableRow (Variables|Combat|GetWeapons) "AK-47")
      (:then
        (Default|SetWeaponinSlot (Variables|Default|GetInventory) _returnvalue "NewEnumerator2")))))

(event Input|KeyboardEvents|V
  (params (Key :type Key%20Structure :default "None"))
  ;[0.01932 0 0.15 0.5] TEMPORARY Assign weapons in inventory
  (:Released
    (bind _returnvalue (Utilities|GetDataTableRow (Variables|Combat|GetWeapons) "Hammer")
      (:then
        (Default|SetWeaponinSlot (Variables|Default|GetInventory) _returnvalue "NewEnumerator3")))))

(event Input|KeyboardEvents|B
  (params (Key :type Key%20Structure :default "None"))
  ;[0.01932 0 0.15 0.5] TEMPORARY Assign weapons in inventory
  (:Released
    (bind _returnvalue (Utilities|GetDataTableRow (Variables|Combat|GetWeapons) "Glock")
      (:then
        (Default|SetWeaponinSlot (Variables|Default|GetInventory) _returnvalue "NewEnumerator1")))))

(fn ConstructionScript)

(fn EquipWeaponbyType
  (params (WeaponType :type E_WeaponType%20Enum :default "NewEnumerator0"))
  (bind _weapon (Default|GetWeaponbyType (Variables|Default|GetInventory) WeaponType))
  (Variables|Combat|SetPendingWeapon _weapon))

(fn GetWeaponMeshbyType
  (params (Type :type E_WeaponType%20Enum :default "NewEnumerator0"))
  (switch Utilities|FlowControl|Switch|SwitchonE_WeaponType Type
    (:NewEnumerator1
      (return (Variables|Default|GetGun)))
    (:NewEnumerator2
      (return (Variables|Default|GetRifle)))
    (:NewEnumerator3
      (return (Variables|Default|GetMeleeWeapon)))))

(fn EquipNewWeapon
  (params (Weapon%20Name :type Weapon%20Data%20Structure))
  (bind (_type _name _attackmontage _damage _speed _mesh _drawmontage _sheathemontage _equippedsocket _unequippedsocket) (Utilities|Struct|BreakWeaponData Weapon%20Name))
  (bind _weapon_mesh (CallFunction|GetWeaponMeshbyType _type))
  (Transformation|AttachComponentToComponent _weapon_mesh (Variables|Character|GetMesh) _unequippedsocket "SnapToTarget" "SnapToTarget" "SnapToTarget" true)
  (Components|StaticMesh|SetStaticMesh _weapon_mesh _mesh))

(fn TakeDamage
  (params (Damage :type Float%20%28double-precision%29))
  (Class|AAAHealthSystemComponent|ReduceHealth (Variables|Default|GetAAA_HealthSystem) Damage)
  (Animation|PlayAnimMontage "/Game/Player/Animations/PlayerHit_Montage.PlayerHit_Montage" 1.0 "None"))