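; BP_Fog is a fog effect actor that feeds the player's position to its FogEffect component as the fog-clearing origin.
; The construction script passes the exposed SpawnRate variable into the effect.
; BeginPlay caches the player pawn as BP_Player, and Tick writes its location to the effect's Clear Fog Origin parameter every frame.
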(event EventBeginPlay
  (bind _asbp_player (Utilities|Casting|CastToBP_Player (Game|Player|GetPlayerPawn 0)))
  (Variables|Default|SetPlayer _asbp_player))

(event Collision|EventActorBeginOverlap
  (params (OtherActor :type Actor%20Object%20Reference)))

(event EventTick
  (params (DeltaSeconds :type Float%20%28single-precision%29))
  (Niagara|SetNiagaraVariable(Vector3) (Variables|Default|GetFogEffect) "Clear Fog Origin" (Transformation|GetActorLocation (Variables|Default|GetPlayer))))

(fn ConstructionScript
  (Niagara|SetNiagaraVariable(Float) (Variables|Default|GetFogEffect) "SpawnRate" (Variables|Default|GetSpawn%20Rate)))